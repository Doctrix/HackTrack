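; Construction-script Blueprint that builds a configurable wire along a spline from spline mesh components.
; SplineMeshVar chooses between one segment per spline point pair and segments at fixed Spacing with scaled direction tangents.
; WireVar selects among six component variants, with the last three taking a second material slot.
; Each segment gets uniform WireSize scaling and dynamic MI_Wire instances driven by color, dirt, specular, roughness and TextureVar texture sets.
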(fn ConstructionScript
  (|Wire))