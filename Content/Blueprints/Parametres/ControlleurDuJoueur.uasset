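; Player controller that centralizes save/load, menu navigation, scoreboard and display settings for a game with levels, music tracks and scores.
; Menu events clear all widgets and show lazily created ones; Tab toggles pause with the scoreboard, and Z also opens the end-of-game menu.
; Player and level data use one save slot; scores append to another, reusing the same SauvegardeDuJeu variable.
; Display options apply through console commands.
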(event Custom|NouvellePartie
  ;[1 1 1] Sauvegarder / Charger
  (bind _returnvalue (SaveGame|CreateSaveGameObject "/Game/Blueprints/Parametres/SauvegardeDuJeu.SauvegardeDuJeu_C"))
  (Variables|Sauvegarde|SetSauvegardeDuJeu _returnvalue))

(event Custom|SauvergarderLeJeu
  (bind _donneesduniveauencours (Variables|Donnees|GetDonneesDuNiveauEnCours))
  ;[1 1 1] Sauvegarder / Charger
  (bind _returnvalue (Game|GetCurrentLevelName true))
  (Variables|/Game/Blueprints/Parametres/SauvegardeDuJeu.SauvegardeDuJeu_C|SetDonneesDuNIveau (Variables|Sauvegarde|GetSauvegardeDuJeu) (Utilities|Struct|Makes_DonneesDuNiveau (Utilities|Array|MakeArray (Utilities|Array|Get(acopy) (.niveau _donneesduniveauencours) (Math|Conversions|ToInteger(Byte) _returnvalue))) (.nomduniveau _donneesduniveauencours) (.scoreàatteindre _donneesduniveauencours) (.titredelamusique _donneesduniveauencours) (.pisteaudio _donneesduniveauencours) (.etatdujeu _donneesduniveauencours)))
  (Variables|/Game/Blueprints/Parametres/SauvegardeDuJeu.SauvegardeDuJeu_C|SetDonneesDuJoueur (Variables|Sauvegarde|GetSauvegardeDuJeu) (Variables|Donnees|GetDonneesDuJoueurEnJeu))
  (SaveGame|SaveGametoSlot (Variables|Sauvegarde|GetSauvegardeDuJeu) "Sauvegarde"))

(event Custom|MenuJouer
  ;[1 1 1] Les menus
  (Viewport|RemoveAllWidgets)
  (Utilities|IsValid (Variables|Widgets|Menu|Getw_MenuJouer)
    (:Is%20Valid
      _)
    (:Is%20Not%20Valid
      (bind _returnvalue (UserInterface|CreateWidget "/Game/Blueprints/Widgets/Menu/MenuJouer.MenuJouer_C"))
      (bind _output_get (Variables|Widgets|Menu|Setw_MenuJouer _returnvalue))))
  (UserInterface|Viewport|AddtoViewport _output_get 0))

(event Custom|AppliquerLesReglagesOptionsAffichage
  (params (Qualite :type e_QualitéParametres%20Enum :default "NewEnumerator0") (ModeDeFenetre :type Boolean) (V_Sync :type Boolean) (QualiteDeLaResolution :type Integer) (Resolution :type String))
  ;[1 1 1] Les reglages options
  (Utilities|FlowControl|Sequence
    (:then_0
      (switch Utilities|FlowControl|Switch|Switchone_QualitéParametres Qualite
        (:NewEnumerator0
          ;;[1 1 1] A corrigé A voir si faut le garder
          (Development|ExecuteConsoleCommand "sg.ViewDistanceQuality 0" 0)
          (Development|ExecuteConsoleCommand "sg.AntiAliasingQuality 0" 0)
          (Development|ExecuteConsoleCommand "sg.PostProcessQuality 0" 0)
          (Development|ExecuteConsoleCommand "sg.ShadowQuality 0" 0)
          (Development|ExecuteConsoleCommand "sg.TextureQuality 0" 0)
          (Development|ExecuteConsoleCommand "sg.EffectsQuality 0" 0)
          (Development|ExecuteConsoleCommand "sg.FoliageQuality 0" 0)
          (Development|ExecuteConsoleCommand "sg.ShadingQuality 0" 0))
        (:NewEnumerator1
          (Development|ExecuteConsoleCommand "sg.ViewDistanceQuality 1" 0)
          (Development|ExecuteConsoleCommand "sg.AntiAliasingQuality 1" 0)
          (Development|ExecuteConsoleCommand "sg.PostProcessQuality 1" 0)
          (Development|ExecuteConsoleCommand "sg.ShadowQuality 1" 0)
          (Development|ExecuteConsoleCommand "sg.TextureQuality 1" 0)
          (Development|ExecuteConsoleCommand "sg.EffectsQuality 1" 0)
          (Development|ExecuteConsoleCommand "sg.FoliageQuality 1" 0)
          (Development|ExecuteConsoleCommand "sg.ShadingQuality 1" 0))
        (:NewEnumerator2
          (Development|ExecuteConsoleCommand "sg.ViewDistanceQuality 2" 0)
          (Development|ExecuteConsoleCommand "sg.AntiAliasingQuality 2" 0)
          (Development|ExecuteConsoleCommand "sg.PostProcessQuality 2" 0)
          (Development|ExecuteConsoleCommand "sg.ShadowQuality 2" 0)
          (Development|ExecuteConsoleCommand "sg.TextureQuality 2" 0)
          (Development|ExecuteConsoleCommand "sg.EffectsQuality 2" 0)
          (Development|ExecuteConsoleCommand "sg.FoliageQuality 2" 0)
          (Development|ExecuteConsoleCommand "sg.ShadingQuality 2" 0))
        (:NewEnumerator3
          (Development|ExecuteConsoleCommand "sg.ViewDistanceQuality 3" 0)
          (Development|ExecuteConsoleCommand "sg.AntiAliasingQuality 3" 0)
          (Development|ExecuteConsoleCommand "sg.PostProcessQuality 3" 0)
          (Development|ExecuteConsoleCommand "sg.ShadowQuality 3" 0)
          (Development|ExecuteConsoleCommand "sg.TextureQuality 3" 0)
          (Development|ExecuteConsoleCommand "sg.EffectsQuality 3" 0)
          (Development|ExecuteConsoleCommand "sg.FoliageQuality 3" 0)
          (Development|ExecuteConsoleCommand "sg.ShadingQuality 3" 0))
        (:NewEnumerator4
          (Development|ExecuteConsoleCommand "sg.ViewDistanceQuality 4" 0)
          (Development|ExecuteConsoleCommand "sg.AntiAliasingQuality 4" 0)
          (Development|ExecuteConsoleCommand "sg.PostProcessQuality 4" 0)
          (Development|ExecuteConsoleCommand "sg.ShadowQuality 4" 0)
          (Development|ExecuteConsoleCommand "sg.TextureQuality 4" 0)
          (Development|ExecuteConsoleCommand "sg.EffectsQuality 4" 0)
          (Development|ExecuteConsoleCommand "sg.FoliageQuality 4" 0)
          (Development|ExecuteConsoleCommand "sg.ShadingQuality 4" 0))))
    (:then_1
      (if ModeDeFenetre
        (Development|ExecuteConsoleCommand (Utilities|String|Append "r.SetRes " Resolution " f") 0)
        (else
          (Development|ExecuteConsoleCommand (Utilities|String|Append "r.SetRes " Resolution " w") 0))))
    (:then_2
      (if V_Sync
        (Development|ExecuteConsoleCommand (Utilities|String|Append "r.VSync " "1") 0)
        (else
          (Development|ExecuteConsoleCommand (Utilities|String|Append "r.VSync " "0") 0))))
    (:then_3
      (Development|ExecuteConsoleCommand (Utilities|String|Append "sg.ResolutionQuality " (Utilities|String|ToString(Integer) QualiteDeLaResolution)) 0))))

(event Custom|MajDesScoresDesJoueurs
  ;[1 1 1] Les menus
  ;;[1 1 1] Score joueur
  (bind _returnvalue (SaveGame|DoesSaveGameExist "SauvegardeScore"))
  (if _returnvalue
    (bind _returnvalue_2 (SaveGame|LoadGamefromSlot "SauvegardeScore"))
    (bind _assauvegarde_du_jeu (Utilities|Casting|CastToSauvegardeDuJeu _returnvalue_2))
    (bind _output_get (Variables|Sauvegarde|SetSauvegardeDuJeu _assauvegarde_du_jeu))
    (Utilities|Array|Add (Variables|/Game/Blueprints/Parametres/SauvegardeDuJeu.SauvegardeDuJeu_C|GetStatsDesJoueurs _output_get) (Variables|Donnees|GetDonneesDuJoueurEnJeu))
    (SaveGame|SaveGametoSlot (Variables|Sauvegarde|GetSauvegardeDuJeu) "SauvegardeScore")
    (else
      (bind _returnvalue_3 (SaveGame|CreateSaveGameObject "/Game/Blueprints/Parametres/SauvegardeDuJeu.SauvegardeDuJeu_C"))
      (bind _assauvegarde_du_jeu_2 (Utilities|Casting|CastToSauvegardeDuJeu _returnvalue_3))
      (bind _output_get_2 (Variables|Sauvegarde|SetSauvegardeDuJeu _assauvegarde_du_jeu_2))
      (Utilities|Array|Add (Variables|/Game/Blueprints/Parametres/SauvegardeDuJeu.SauvegardeDuJeu_C|GetStatsDesJoueurs _output_get_2) (Variables|Donnees|GetDonneesDuJoueurEnJeu))
      (SaveGame|SaveGametoSlot (Variables|Sauvegarde|GetSauvegardeDuJeu) "SauvegardeScore")))
  (CallFunction|TableauDesScores))

(event Custom|TableauDesScores
  (bind _returnvalue (Viewport|GetViewportSize))
  ;[1 1 1] Les menus
  (bind _returnvalue_2 (UserInterface|CreateWidget "/Game/Blueprints/Widgets/HUD/TableauDesScores.TableauDesScores_C"))
  (Variables|Widgets|Setw_TableauDesScores _returnvalue_2)
  (Class|UserWidget|SetAlignmentinViewport _returnvalue_2 "(X=0.500000,Y=0.500000)")
  (Class|UserWidget|SetAnchorsinViewport _returnvalue_2 (Utilities|Struct|MakeAnchors "(X=0.500000,Y=0.500000)" "(X=0.500000,Y=0.500000)"))
  (Class|UserWidget|SetPositioninViewport _returnvalue_2 (Math|Vector2D|MakeVector2D (/ (.x _returnvalue) 2.0) (/ (.y _returnvalue) 2.0)) true)
  (Class|UserWidget|SetDesiredSizeinViewport _returnvalue_2 "(X=1280.000000,Y=720.000000)")
  (UserInterface|Viewport|AddtoViewport _returnvalue_2 0)
  (Default|AjouterUnJoueur (Variables|Widgets|Getw_TableauDesScores) 0 (Variables|/Game/Blueprints/Parametres/SauvegardeDuJeu.SauvegardeDuJeu_C|GetStatsDesJoueurs (Variables|Sauvegarde|GetSauvegardeDuJeu)) false))

(event Custom|EnregistrementInfosJoueur
  (bind _returnvalue (Viewport|GetViewportSize))
  ;[1 1 1] Les menus
  (if (not (Variables|/Game/Blueprints/Widgets/Menu/MenuPrincipale.MenuPrincipale_C|GetJoueurEstEnregistrer? (Variables|Widgets|Menu|Getw_MenuPrincipal)))
    (Utilities|FlowControl|DoOnce false
      (:Completed
        (Viewport|RemoveAllWidgets)
        (bind _returnvalue_2 (UserInterface|CreateWidget "/Game/Blueprints/Widgets/HUD/EnregistrementInfos.EnregistrementInfos_C"))
        (Class|UserWidget|SetAlignmentinViewport _returnvalue_2 "(X=0.500000,Y=0.500000)")
        (Class|UserWidget|SetAnchorsinViewport _returnvalue_2 (Utilities|Struct|MakeAnchors "(X=0.500000,Y=0.500000)" "(X=0.500000,Y=0.500000)"))
        (Class|UserWidget|SetPositioninViewport _returnvalue_2 (Math|Vector2D|MakeVector2D (/ (.x _returnvalue) 2.0) (/ (.y _returnvalue) 2.0)) true)
        (Class|UserWidget|SetDesiredSizeinViewport _returnvalue_2 "(X=700.000000,Y=300.000000)")
        (UserInterface|Viewport|AddtoViewport _returnvalue_2 0)
        (Variables|Widgets|Setw_EnregistrementInfoDuJoueur _returnvalue_2)))))

(event Custom|AfficherTableauDesScores
  (bind _w_tableaudesscores (Variables|Widgets|Getw_TableauDesScores))
  (if (Variables|Default|GetTableauDesScoresAfficher)
    (Utilities|IsValid _w_tableaudesscores
      (:Is%20Valid
        (UserInterface|Viewport|AddtoViewport _w_tableaudesscores 0)))
    (else
      (Variables|Default|SetTableauDesScoresAfficher true)
      (CallFunction|MajDesScoresDesJoueurs))))

(event Custom|MenuPrincipal
  ;[1 1 1] Les menus
  (Viewport|RemoveAllWidgets)
  (Utilities|IsValid (Variables|Widgets|Menu|Getw_MenuPrincipal)
    (:Is%20Valid
      _)
    (:Is%20Not%20Valid
      (bind _returnvalue (UserInterface|CreateWidget "/Game/Blueprints/Widgets/Menu/MenuPrincipale.MenuPrincipale_C"))
      (bind _output_get (Variables|Widgets|Menu|Setw_MenuPrincipal _returnvalue))))
  (UserInterface|Viewport|AddtoViewport _output_get 0))

(event Custom|MenuPause
  ;[1 1 1] Les menus
  (Viewport|RemoveAllWidgets)
  (Utilities|IsValid (Variables|Widgets|Menu|Getw_MenuPause)
    (:Is%20Valid
      _)
    (:Is%20Not%20Valid
      (bind _returnvalue (UserInterface|CreateWidget "/Game/Blueprints/Widgets/Menu/MenuPause.MenuPause_C"))
      (bind _output_get (Variables|Widgets|Menu|Setw_MenuPause _returnvalue))))
  (UserInterface|Viewport|AddtoViewport _output_get 0))

(event Custom|MenuOptions
  ;[1 1 1] Les menus
  (Viewport|RemoveAllWidgets)
  (Utilities|IsValid (Variables|Widgets|Menu|Getw_MenuOptions)
    (:Is%20Valid
      _)
    (:Is%20Not%20Valid
      (bind _returnvalue (UserInterface|CreateWidget "/Game/Blueprints/Widgets/Menu/MenuOptions.MenuOptions_C"))
      (bind _output_get (Variables|Widgets|Menu|Setw_MenuOptions _returnvalue))))
  (UserInterface|Viewport|AddtoViewport _output_get 0))

(event Custom|AfficherInterfaceDuJoueur
  ;[1 1 1] Interface du joueur
  (Viewport|RemoveAllWidgets)
  (Utilities|IsValid (Variables|Widgets|IU|GetInterfaceDuJoueur)
    (:Is%20Valid
      _)
    (:Is%20Not%20Valid
      (bind _returnvalue (UserInterface|CreateWidget "/Game/Blueprints/Widgets/InterfaceDuJoueur.InterfaceDuJoueur_C"))
      (bind _output_get (Variables|Widgets|IU|SetInterfaceDuJoueur _returnvalue))))
  (UserInterface|Viewport|AddtoViewport _output_get 0)
  (Variables|Default|SetbShowMouseCursor false)
  (Input|SetInputModeGameandUI self 0 "LockAlways" true))

(event Custom|MenuDeFinDePartie
  (params (ObjectifAtteint :type Boolean))
  ;[1 1 1] Les menus
  (Viewport|RemoveAllWidgets)
  (Utilities|IsValid (Variables|Widgets|Menu|Getw_MenuDeFinDePartie)
    (:Is%20Valid
      _)
    (:Is%20Not%20Valid
      (bind _returnvalue (UserInterface|CreateWidget "/Game/Blueprints/Widgets/Menu/MenuFinDePartie.MenuFinDePartie_C"))
      (bind _output_get (Variables|Widgets|Menu|Setw_MenuDeFinDePartie _returnvalue))))
  (UserInterface|Viewport|AddtoViewport _output_get 0)
  (Default|TexteDeFin _output_get)
  (CallFunction|AfficherTableauDesScores)
  (Variables|/Game/Blueprints/Widgets/Menu/MenuFinDePartie.MenuFinDePartie_C|SetObjectifAtteint _output_get ObjectifAtteint)
  (Variables|Conditions|SetFinDuJeu true))

(event Custom|MenuPlaylist
  ;[1 1 1] Les menus
  (Viewport|RemoveAllWidgets)
  (Utilities|IsValid (Variables|Widgets|IU|GetInterfaceDuJoueur)
    (:Is%20Valid
      _)
    (:Is%20Not%20Valid
      (bind _returnvalue (UserInterface|CreateWidget "/Game/Blueprints/Widgets/Menu/MenuPlaylist.MenuPlaylist_C"))
      (bind _output_get (Variables|Widgets|Menu|Setw_MenuPlaylist _returnvalue))))
  (UserInterface|Viewport|AddtoViewport _output_get 0))

(event Custom|ChargerLeJeu
  ;[1 1 1] Sauvegarder / Charger
  (bind _returnvalue (SaveGame|DoesSaveGameExist "Sauvegarde"))
  (if _returnvalue
    (bind _returnvalue_2 (SaveGame|LoadGamefromSlot "Sauvegarde"))
    (bind _assauvegarde_du_jeu (Utilities|Casting|CastToSauvegardeDuJeu _returnvalue_2))
    (bind _output_get (Variables|Sauvegarde|SetSauvegardeDuJeu _assauvegarde_du_jeu))
    (Variables|Donnees|SetDonneesDuJoueurEnJeu (Variables|/Game/Blueprints/Parametres/SauvegardeDuJeu.SauvegardeDuJeu_C|GetDonneesDuJoueur _output_get))
    (Variables|Donnees|SetDonneesDuNiveauEnCours (Variables|/Game/Blueprints/Parametres/SauvegardeDuJeu.SauvegardeDuJeu_C|GetDonneesDuNIveau _output_get))
    (else
      (CallFunction|NouvellePartie))))

(event Input|KeyboardEvents|Tab
  (params (Key :type Key%20Structure :default "None"))
  (bind _w_tableaudesscores (Variables|Widgets|Getw_TableauDesScores))
  (:Pressed
    (bind _isa (Utilities|FlowControl|FlipFlop)
      (:A
        _)
      (:B
        _))
    (bind _returnvalue (Game|SetGamePaused _isa))
    (if _returnvalue
      (CallFunction|AfficherTableauDesScores)
      (Variables|/Script/Engine.PlayerController|SetbShowMouseCursor (Game|GetPlayerController 0) true)
      (else
        (Utilities|IsValid _w_tableaudesscores
          (:Is%20Valid
            (Widget|RemovefromParent _w_tableaudesscores)
            (Variables|/Script/Engine.PlayerController|SetbShowMouseCursor (Game|GetPlayerController 0) false)))))))

(event Input|KeyboardEvents|Z
  (params (Key :type Key%20Structure :default "None"))
  ;[1 1 1] Les menus
  (:Pressed
    (Viewport|RemoveAllWidgets)
    (Utilities|IsValid (Variables|Widgets|Menu|Getw_MenuDeFinDePartie)
      (:Is%20Valid
        _)
      (:Is%20Not%20Valid
        (bind _returnvalue (UserInterface|CreateWidget "/Game/Blueprints/Widgets/Menu/MenuFinDePartie.MenuFinDePartie_C"))
        (bind _output_get (Variables|Widgets|Menu|Setw_MenuDeFinDePartie _returnvalue))))
    (UserInterface|Viewport|AddtoViewport _output_get 0)
    (Default|TexteDeFin _output_get)
    (CallFunction|AfficherTableauDesScores)
    (Variables|/Game/Blueprints/Widgets/Menu/MenuFinDePartie.MenuFinDePartie_C|SetObjectifAtteint _output_get (stale Custom|MenuDeFinDePartie ObjectifAtteint))
    (Variables|Conditions|SetFinDuJeu true)))

(fn ConstructionScript)