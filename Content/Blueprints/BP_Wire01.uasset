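; BP_Wire01 is a configurable wire actor that builds spline meshes along its Spline in the construction script.
; SplineMeshVar selects segments between spline points or at fixed Spacing with scaled tangents.
; WireVar picks one of six mesh component variants, each scaled by WireSize.
; Each segment gets dynamic MI_Wire instances on one or two material slots, driven by color, dirt, specular, roughness and a selectable texture set.
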(fn ConstructionScript
  (|Wire))