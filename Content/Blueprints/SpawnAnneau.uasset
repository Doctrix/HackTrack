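; SpawnAnneau is a spawner actor that places a ring (anneau) at its own location and rotation when play begins.
; BeginPlay calls VerifierAnneauSurLaCarte, which runs SpawnAnneau whether or not a current ring is valid.
; The TypeObstacle macro checks the obstacle type and spawns the class indexed by NumeroType in the Anneau array.
; The spawned ring is stored in AnneauEnCours.
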(event EventBeginPlay
  (CallFunction|VerifierAnneauSurLaCarte "NewEnumerator0"))

(event Collision|EventActorBeginOverlap
  (params (OtherActor :type Actor%20Object%20Reference)))

(fn ConstructionScript)

(fn VerifierAnneauSurLaCarte
  (params (type :type e_type%20Enum :default "NewEnumerator4") (NumeroType :type Integer))
  (Utilities|IsValid (Variables|Default|GetAnneauEnCours)
    (:Is%20Valid
      _)
    (:Is%20Not%20Valid
      _))
  (CallFunction|SpawnAnneau type NumeroType))

(fn SpawnAnneau
  (params (type :type e_type%20Enum :default "NewEnumerator4") (NumeroType :type Integer))
  (bind _obstacle (Utilities|TypeObstacle (Math|Transform|MakeTransform (Transformation|GetActorLocation) (Transformation|GetActorRotation)) type NumeroType)
    (:then
      (Variables|Default|SetAnneauEnCours _obstacle))))