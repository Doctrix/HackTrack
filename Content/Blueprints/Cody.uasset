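; Cody is a player-input Blueprint that scores points by destroying rings (Anneau, of class Platform) on the Action input.
; CastsRef grabs the first Platform found in the level, refreshed at BeginPlay and on each press.
; If that ring's EntrerDansLaZone flag is set, the press destroys it, increments Score and updates the HUD.
; ActionActiver tracks the press, clearing on a score, on release, or after a delay when no ring exists.
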(event EventBeginPlay
  (Utilities|CastsRef)
  (bind _as0_hud (Utilities|Casting|CastTo0_HUD (HUD|GetHUD (Game|GetPlayerController 0))))
  (Variables|Default|SetHUD _as0_hud))

(event Collision|EventActorBeginOverlap
  (params (OtherActor :type Actor%20Object%20Reference)))

(event EventTick
  (params (DeltaSeconds :type Float%20%28single-precision%29)))

(event Input|ActionEvents|InputActionAction
  (params (Key :type Key%20Structure :default "None"))
  (bind _anneau (Variables|Default|GetAnneau))
  (:Pressed
    (Variables|Default|SetActionActiver true)
    (Utilities|CastsRef)
    (Utilities|IsValid _anneau
      (:Is%20Valid
        (if (Variables|/Game/Blueprints/Platform.Platform_C|GetEntrerDansLaZone _anneau)
          (Default|Detruire _anneau)
          (Variables|Default|SetScore (+ (Variables|Default|GetScore) 1))
          (Default|MajDuScore (Variables|/Game/Blueprints/0_HUD.0_HUD_C|GetInterfaceDuJoueur (Variables|Default|GetHUD)) (Utilities|Text|ToText(Integer) (Variables|Default|GetScore)))
          (Variables|Default|SetActionActiver false :!label _label)))
      (:Is%20Not%20Valid
        (Utilities|FlowControl|Delay 1.0)
        (goto _label))))
  (:Released
    (if (Variables|Default|GetActionActiver)
      (Variables|Default|SetActionActiver false))))

(fn ConstructionScript)