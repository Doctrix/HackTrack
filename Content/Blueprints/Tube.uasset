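; Tube segment actor that prompts the game mode to spawn another tube when the player passes through it.
; A Box overlap by Cody calls SpawnTube on ModeDeJeu and prints a debug message, with no guard against repeat triggers.
; The construction script fills SpawnPoints with the relative transforms of five placement components, though this file does not use the array further.
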(event OnComponentBeginOverlap(Box)
  (params (OverlappedComponent :type Primitive%20Component%20Object%20Reference) (OtherActor :type Actor%20Object%20Reference) (OtherComp :type Primitive%20Component%20Object%20Reference) (OtherBodyIndex :type Integer) (bFromSweep :type Boolean) (SweepResult :type Hit%20Result%20Structure%20%28by%20ref%29))
  (Utilities|Casting|CastToCody OtherActor)
  (bind _asmode_de_jeu (Utilities|Casting|CastToModeDeJeu (Game|GetGameMode)))
  (Default|SpawnTube _asmode_de_jeu)
  (Development|PrintString "Spawn tube"))

(event EventBeginPlay)

(event Collision|EventActorBeginOverlap
  (params (OtherActor :type Actor%20Object%20Reference)))

(event EventTick
  (params (DeltaSeconds :type Float%20%28single-precision%29)))

(fn ConstructionScript
  (CallFunction|SetSpawnPoints))

(fn SetSpawnPoints
  (Variables|Default|SetSpawnPoints (Utilities|Array|MakeArray (Transformation|GetRelativeTransform (Variables|Default|GetEmpl_G)) (Transformation|GetRelativeTransform (Variables|Default|GetEmpl_AG)) (Transformation|GetRelativeTransform (Variables|Default|GetEmpl_AD)) (Transformation|GetRelativeTransform (Variables|Default|GetEmpl_D)) (Transformation|GetRelativeTransform (Variables|Default|GetEmpl_C)))))