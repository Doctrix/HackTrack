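; Cody is the player character, moving forward automatically during the game and scoring by destroying rings with the Action input.
; Tick updates HUD gauges, moves the Sphere and doubles its speed after each long Delay.
; Action zooms the spring arm and rewards the first Anneau_Principal found, if entered.
; Timelines swing the camera back and forth and vary zoom per spawned obstacle type, while CouleurDuKarma swaps the aura particles.
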(event Custom|CouleurDuKarma
  (params (Particles :type Particle%20System%20Object%20Reference))
  (Effects|Components|ParticleSystem|SetTemplate (Variables|Default|GetAura) Particles))

(event EventBeginPlay
  (bind _ascontrolleur_du_joueur (Utilities|CastsControlleurDuJoueur))
  (bind _as0_hud (Utilities|Casting|CastTo0_HUD (HUD|GetHUD _ascontrolleur_du_joueur)))
  (Variables|Default|SetHUD _as0_hud)
  (Utilities|AnneauPrincipalRef))

(event EventTick
  (params (DeltaSeconds :type Float%20%28single-precision%29))
  (bind _ascontrolleur_du_joueur (Utilities|CastsControlleurDuJoueur))
  (if (Variables|/Game/Blueprints/Parametres/ControlleurDuJoueur.ControlleurDuJoueur_C|GetDebutDuJeu _ascontrolleur_du_joueur)
    (if (not (Variables|/Game/Blueprints/Parametres/ControlleurDuJoueur.ControlleurDuJoueur_C|GetFinDuJeu _ascontrolleur_du_joueur))
      (bind _ascontrolleur_du_joueur_2 (Utilities|CastsControlleurDuJoueur))
      (Utilities|IsValid (Variables|/Game/Blueprints/Parametres/ControlleurDuJoueur.ControlleurDuJoueur_C|GetInterfaceDuJoueur _ascontrolleur_du_joueur_2)
        (:Is%20Valid
          (CallFunction|Jauge (Variables|/Game/Blueprints/Parametres/ControlleurDuJoueur.ControlleurDuJoueur_C|GetInterfaceDuJoueur _ascontrolleur_du_joueur_2))
          (|Rotationdelacamera)
          ;[1 1 1] Vitesse de deplacement
          (Transformation|AddRelativeLocation (Variables|Default|GetSphere) (Math|Vector|MakeVector (Variables|Details|GetVitesseDeDeplacement) 0.0 0.0) false false)
          (Utilities|FlowControl|Delay 2e+02)
          (if (Variables|Conditions|GetMultiplieActiver) :!label _label
            (Variables|Conditions|SetMultiplieActiver false)
            (bind _output_get (Variables|Details|SetVitesseDeDeplacement (* (Variables|Details|GetVitesseDeDeplacement) 2.0)))
            (Development|PrintString (Utilities|String|ToString(Float) _output_get))
            (else
              (Variables|Details|SetVitesseDeDeplacement (Variables|Details|GetVitesseDeDeplacement))
              (Variables|Conditions|SetMultiplieActiver true)
              (goto _label))))))))

(event Input|ActionEvents|InputActionAction
  (params (Key :type Key%20Structure :default "None"))
  (bind _springarm (Variables|Default|GetSpringArm))
  (bind _anneau (Variables|Default|GetAnneau))
  ;[1 1 1] Possibliter de creer une fonction /""
  (:Pressed
    ;;[1 1 1] Action appui long duree 1 seconde
    (bind _zoom (Timeline|Zoom Play)
      (:Update
        (Variables|/Script/Engine.SpringArmComponent|SetTargetArmLength _springarm _zoom)
        (Variables|Conditions|SetActionActiver true)
        (bind _ascontrolleur_du_joueur (Utilities|CastsControlleurDuJoueur))
        (Appearance|SetColorandOpacity (Variables|/Game/Blueprints/Widgets/InterfaceDuJoueur.InterfaceDuJoueur_C|GetNotificationManette (Variables|/Game/Blueprints/Parametres/ControlleurDuJoueur.ControlleurDuJoueur_C|GetInterfaceDuJoueur _ascontrolleur_du_joueur)) "(R=0.000000,G=0.562500,B=0.100505,A=1.000000)" :!class /Script/UMG.UserWidget)
        (Appearance|SetColorandOpacity (Variables|/Game/Blueprints/Widgets/InterfaceDuJoueur.InterfaceDuJoueur_C|GetIndicationToucheClavier (Variables|/Game/Blueprints/Parametres/ControlleurDuJoueur.ControlleurDuJoueur_C|GetInterfaceDuJoueur _ascontrolleur_du_joueur)) (Utilities|Struct|MakeSlateColor "(R=0.000000,G=0.333333,B=0.059558,A=1.000000)" "UseColor_Specified") :!class /Script/UMG.TextBlock)
        (Utilities|AnneauPrincipalRef)
        (Utilities|IsValid _anneau
          (:Is%20Valid
            (if (Variables|Conditions|GetActionActiver)
              (if (Variables|/Game/Blueprints/Anneau_Principal.Anneau_Principal_C|GetEntrerDansLaZone _anneau)
                (bind _ascontrolleur_du_joueur_2 (Utilities|CastsControlleurDuJoueur))
                (CallFunction|StatistiquesDuJoueur (Variables|/Game/Blueprints/Parametres/ControlleurDuJoueur.ControlleurDuJoueur_C|GetInterfaceDuJoueur _ascontrolleur_du_joueur_2) (Variables|Default|GetAnneau)))))))))
  (:Released
    (bind _zoom_2 (Timeline|Dezoom Play)
      (:Update
        (Variables|/Script/Engine.SpringArmComponent|SetTargetArmLength _springarm _zoom_2)
        (bind _ascontrolleur_du_joueur_3 (Utilities|CastsControlleurDuJoueur))
        (Appearance|SetColorandOpacity (Variables|/Game/Blueprints/Widgets/InterfaceDuJoueur.InterfaceDuJoueur_C|GetNotificationManette (Variables|/Game/Blueprints/Parametres/ControlleurDuJoueur.ControlleurDuJoueur_C|GetInterfaceDuJoueur _ascontrolleur_du_joueur_3)) "(R=1.000000,G=1.000000,B=1.000000,A=1.000000)" :!class /Script/UMG.UserWidget)
        (Appearance|SetColorandOpacity (Variables|/Game/Blueprints/Widgets/InterfaceDuJoueur.InterfaceDuJoueur_C|GetIndicationToucheClavier (Variables|/Game/Blueprints/Parametres/ControlleurDuJoueur.ControlleurDuJoueur_C|GetInterfaceDuJoueur _ascontrolleur_du_joueur_3)) (Utilities|Struct|MakeSlateColor "(R=1.000000,G=1.000000,B=1.000000,A=1.000000)" "UseColor_Specified") :!class /Script/UMG.TextBlock)))))

(fn ConstructionScript)

(fn StatistiquesDuJoueur
  (params (InterfaceDuJoueur :type Interface%20Du%20Joueur%20Object%20Reference) (Obstacle :type Anneau%20Principal%20Object%20Reference))
  (bind _score (Variables|Details|GetScore))
  (Utilities|IsValid Obstacle
    (:Is%20Valid
      (Default|Recompense Obstacle (Variables|/Game/Blueprints/Anneau_Principal.Anneau_Principal_C|Gettype Obstacle) _score)
      (Default|MajDuScore InterfaceDuJoueur (Utilities|Text|ToText(Integer) _score) 300)
      (Default|Detruire Obstacle))
    (:Is%20Not%20Valid
      _))
  (return))

(fn Jauge
  (params (InterfaceDuJoueur :type Interface%20Du%20Joueur%20Object%20Reference))
  (Default|BarreHumeur InterfaceDuJoueur (Variables|Details|GetHumeur))
  (Default|JaugeDeRalenti InterfaceDuJoueur (Variables|Details|GetRalenti))
  (Default|JaugeDeLecranFlou InterfaceDuJoueur (Variables|Details|GetFlou))
  (Default|JaugeTousEnNORMAL InterfaceDuJoueur (Variables|Details|GetRAS))
  (Default|JaugeSuperSonic InterfaceDuJoueur (Variables|Details|GetSonic))
  (return))

(event Custom|RotationQuandSpawnDanger
  (|TempoDeLaCamera) ; enters at Danger
)

(event Custom|RotationQuandSpawnObstacleNormal
  (|TempoDeLaCamera) ; enters at Normal
)

(event Custom|RotationQuandSpawnObstacleBonus
  (|TempoDeLaCamera) ; enters at Bonus
)

(event Custom|RotationQuandSpawnObstacleBoost
  (|TempoDeLaCamera) ; enters at Boost
)