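; Ring obstacle (Cercle_Principal) in four types (normal, bonus, boost, danger) that drifts along X by a random step each Tick.
; GestionParType applies its material colour and per-type spawn particles.
; Recompense, not called here, adjusts Cody's score and mood/effect gauges, triggering player modes at their limits, plus karma colour, explosion and sound.
; A sphere overlap tracks Cody, and the actor destroys itself two seconds after Cody leaves.
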(event OnComponentBeginOverlap(Sphere)
  (params (OverlappedComponent :type Primitive%20Component%20Object%20Reference) (OtherActor :type Actor%20Object%20Reference) (OtherComp :type Primitive%20Component%20Object%20Reference) (OtherBodyIndex :type Integer) (bFromSweep :type Boolean) (SweepResult :type Hit%20Result%20Structure%20%28by%20ref%29))
  (bind _ascody (Utilities|Casting|CastToCody OtherActor))
  (Variables|Ref|SetPersonnage _ascody)
  (Variables|Conditions|SetEntrerDansLaZone true))

(event OnComponentEndOverlap(Sphere)
  (params (OverlappedComponent :type Primitive%20Component%20Object%20Reference) (OtherActor :type Actor%20Object%20Reference) (OtherComp :type Primitive%20Component%20Object%20Reference) (OtherBodyIndex :type Integer))
  (bind _ascody (Utilities|Casting|CastToCody OtherActor))
  (Variables|Ref|SetPersonnage _ascody)
  (Variables|Conditions|SetEntrerDansLaZone false)
  (if (not (Variables|Conditions|GetEntrerDansLaZone))
    (Utilities|FlowControl|Delay 2.0)
    (CallFunction|Detruire)))

(event Custom|FX_Explosion
  (params (NewTemplate :type Particle%20System%20Object%20Reference))
  (Effects|Components|ParticleSystem|SetTemplate (Variables|/Game/Blueprints/Personnages/Cody.Cody_C|GetParticleSystem (Variables|Ref|GetPersonnage)) NewTemplate))

(event Custom|Detruire
  (Components|Activation|SetAutoActivate (Variables|Default|GetParticleSystem) true)
  (Actor|DestroyActor))

(event Custom|FXapparitionObstacle
  (params (NewTemplate :type Particle%20System%20Object%20Reference))
  (Effects|Components|ParticleSystem|SetTemplate (Variables|Default|GetParticleSystem) NewTemplate))

(event EventBeginPlay
  (bind _ascody (Utilities|Casting|CastToCody (Game|Player|GetPlayerPawn 0)))
  (Variables|Ref|SetPersonnage _ascody)
  (for _array_element (Utilities|Array|MakeArray (Variables|Default|GetStaticMesh) (Variables|Default|GetStaticMesh1))
    (bind _returnvalue (Rendering|Material|CreateDynamicMaterialInstance _array_element 0 "/Game/Materials/M_Obstacle.M_Obstacle" "None" :!class /Script/Engine.PrimitiveComponent))
    (Variables|Ref|SetMID _returnvalue)
    (CallFunction|GestionParType)))

(event EventTick
  (params (DeltaSeconds :type Float%20%28single-precision%29))
  (Transformation|AddRelativeLocation (Variables|Default|GetAnneau) (Math|Vector|MakeVector (Math|Random|RandomFloatinRange (Variables|Default|GetVitesseDeDeplacementMin) (Variables|Default|GetVitesseDeDeplacementMax)) 0.0 0.0) false false))

(fn ConstructionScript
  (for _array_element (Utilities|Array|MakeArray (Variables|Default|GetStaticMesh) (Variables|Default|GetStaticMesh1))
    (bind _returnvalue (Rendering|Material|CreateDynamicMaterialInstance _array_element 0 "/Game/Materials/M_Obstacle.M_Obstacle" "None" :!class /Script/Engine.PrimitiveComponent))
    (Variables|Ref|SetMID _returnvalue)
    (Rendering|Material|SetVectorParameterValue (Variables|Ref|GetMID) "Couleur" (Variables|Default|GetCouleurMaterial) :!class /Script/Engine.MaterialInstanceDynamic)
    (CallFunction|GestionParType)))

(fn GestionParType
  (bind _mid (Variables|Ref|GetMID))
  (if (Utilities|Enum|Equal(Enum) (Variables|Default|GetTypeCercle) "NewEnumerator0")
    (Rendering|Material|SetVectorParameterValue _mid "Couleur" (Variables|Default|GetCouleurMaterial) :!class /Script/Engine.MaterialInstanceDynamic)
    (CallFunction|FXapparitionObstacle (Variables|FX|GetFxNormal))
    (elif (Utilities|Enum|Equal(Enum) (Variables|Default|GetTypeCercle) "NewEnumerator1")
      (Rendering|Material|SetVectorParameterValue _mid "Couleur" (Variables|Default|GetCouleurMaterial) :!class /Script/Engine.MaterialInstanceDynamic)
      (CallFunction|FXapparitionObstacle (Variables|FX|GetFxBonus))
      (elif (Utilities|Enum|Equal(Enum) (Variables|Default|GetTypeCercle) "NewEnumerator2")
        (Rendering|Material|SetVectorParameterValue _mid "Couleur" (Variables|Default|GetCouleurMaterial) :!class /Script/Engine.MaterialInstanceDynamic)
        (CallFunction|FXapparitionObstacle (Variables|FX|GetFxBoost))
        (elif (Utilities|Enum|Equal(Enum) (Variables|Default|GetTypeCercle) "NewEnumerator3")
          (Rendering|Material|SetVectorParameterValue _mid "Couleur" (Variables|Default|GetCouleurMaterial) :!class /Script/Engine.MaterialInstanceDynamic)
          (CallFunction|FXapparitionObstacle (Variables|FX|GetFxDanger))))))
  (return))

(fn Recompense
  (params (Type :type e_type%20Enum :default "NewEnumerator0") (Montant :type Integer))
  (bind _personnage (Variables|Ref|GetPersonnage))
  (bind _personnage_2 (Variables|Ref|GetPersonnage))
  ;[1 1 1] Normal
  (if (Utilities|Enum|Equal(Enum) Type "NewEnumerator0")
    (CallFunction|AjouterPoints Montant _personnage)
    (CallFunction|Conditions true false)
    (CallFunction|ConditionsCercle true false false false)
    (CallFunction|AjouterHumeur _personnage_2 0.5)
    (CallFunction|AjouterRalenti _personnage_2 0.1)
    (CallFunction|AjouterRAS _personnage_2 0.1)
    (Default|CouleurDuKarma _personnage_2 (Variables|/Game/Blueprints/Personnages/Cody.Cody_C|GetKarma_Normal _personnage_2))
    (CallFunction|FXExplosion self (Variables|FX|GetFxNormal))
    (Audio|SpawnSoundatLocation "/Game/Audio/Tap-01.Tap-01" "0, 0, 0" "0, 0, 0" 0.1 1.0 0.0 0 0)
    (else
      ;[1 1 1] Bonus
      (if (Utilities|Enum|Equal(Enum) Type "NewEnumerator1")
        (CallFunction|AjouterPoints Montant _personnage)
        (CallFunction|Conditions true false)
        (CallFunction|ConditionsCercle false false true false)
        (CallFunction|AjouterHumeur _personnage_2 2.0)
        (CallFunction|AjouterRalenti _personnage_2 1.0)
        (CallFunction|AjouterRAS _personnage_2 1.0)
        (Default|CouleurDuKarma _personnage_2 (Variables|/Game/Blueprints/Personnages/Cody.Cody_C|GetKarma_Bonus _personnage_2))
        (CallFunction|FXExplosion self (Variables|FX|GetFxBonus))
        (Audio|SpawnSoundatLocation "/Game/Audio/Tube-Hit.Tube-Hit" "0, 0, 0" "0, 0, 0" 0.1 1.0 0.0 0 0)
        (else
          ;[1 1 1] Boost
          (if (Utilities|Enum|Equal(Enum) Type "NewEnumerator2")
            (CallFunction|AjouterPoints Montant _personnage)
            (CallFunction|Conditions true false)
            (CallFunction|ConditionsCercle false true false false)
            (CallFunction|AjouterSonic _personnage_2 2.0)
            (Default|ZoomBoost _personnage_2)
            (CallFunction|AjouterRAS _personnage_2 1.0)
            (Default|CouleurDuKarma _personnage_2 (Variables|/Game/Blueprints/Personnages/Cody.Cody_C|GetKarma_Boost _personnage_2))
            (CallFunction|FXExplosion self (Variables|FX|GetFxBonus))
            (Audio|SpawnSoundatLocation "/Game/Audio/Tube-Hit.Tube-Hit" "0, 0, 0" "0, 0, 0" 0.1 1.0 0.0 0 0)
            (else
              ;[1 1 1] Danger
              (if (Utilities|Enum|Equal(Enum) Type "NewEnumerator3")
                (CallFunction|DiminuerPoints Montant _personnage)
                (CallFunction|Conditions true true)
                (CallFunction|ConditionsCercle false false false true)
                (CallFunction|DiminuerHumeur _personnage_2 2.0)
                (CallFunction|AjouterFlou _personnage_2 2.0)
                (CallFunction|AjouterRAS _personnage_2 -1.0)
                (Default|CouleurDuKarma _personnage_2 (Variables|/Game/Blueprints/Personnages/Cody.Cody_C|GetKarma_Danger _personnage_2))
                (CallFunction|FXExplosion self (Variables|FX|GetFxDanger))
                (Audio|SpawnSoundatLocation "/Game/Audio/Tap-02.Tap-02" "0, 0, 0" "0, 0, 0" 0.1 1.0 0.0 0 0)))))))))

(fn AjouterHumeur
  (params (Personnage :type Cody%20Object%20Reference) (Montant :type Float%20%28single-precision%29))
  (if (< (Variables|/Game/Blueprints/Personnages/Cody.Cody_C|GetHumeur Personnage) 1e+02)
    (Variables|/Game/Blueprints/Personnages/Cody.Cody_C|SetHumeur Personnage (+ (Variables|/Game/Blueprints/Personnages/Cody.Cody_C|GetHumeur Personnage) Montant))
    (else
      (Default|ModeBonneHumeur Personnage))))

(fn DiminuerHumeur
  (params (Personage :type Cody%20Object%20Reference) (Montant :type Float%20%28single-precision%29))
  (if (> (Variables|/Game/Blueprints/Personnages/Cody.Cody_C|GetHumeur Personage) 0.0)
    (Variables|/Game/Blueprints/Personnages/Cody.Cody_C|SetHumeur Personage (- (Variables|/Game/Blueprints/Personnages/Cody.Cody_C|GetHumeur Personage) Montant))
    (else
      (Default|ModeMauvaiseHumeur Personage))))

(fn AjouterRalenti
  (params (Personnage :type Cody%20Object%20Reference) (Montant :type Float%20%28single-precision%29))
  (if (< (Variables|/Game/Blueprints/Personnages/Cody.Cody_C|GetRalenti Personnage) 1e+02)
    (Variables|/Game/Blueprints/Personnages/Cody.Cody_C|SetRalenti Personnage (+ (Variables|/Game/Blueprints/Personnages/Cody.Cody_C|GetRalenti Personnage) Montant))
    (else
      (Default|ModeRalenti Personnage))))

(fn AjouterFlou
  (params (Personnage :type Cody%20Object%20Reference) (Montant :type Float%20%28single-precision%29))
  (if (< (Variables|/Game/Blueprints/Personnages/Cody.Cody_C|GetFlou Personnage) 1e+02)
    (Variables|/Game/Blueprints/Personnages/Cody.Cody_C|SetFlou Personnage (+ (Variables|/Game/Blueprints/Personnages/Cody.Cody_C|GetFlou Personnage) Montant))
    (else
      (Default|ModeEcranFlou Personnage))))

(fn AjouterRAS
  (params (Personnage :type Cody%20Object%20Reference) (Montant :type Float%20%28single-precision%29))
  (if (< (Variables|/Game/Blueprints/Personnages/Cody.Cody_C|GetRAS Personnage) 1e+02)
    (Variables|/Game/Blueprints/Personnages/Cody.Cody_C|SetRAS Personnage (+ (Variables|/Game/Blueprints/Personnages/Cody.Cody_C|GetRAS Personnage) Montant))
    (else
      (Default|ModeTousVaBien Personnage))))

(fn AjouterSonic
  (params (Personnage :type Cody%20Object%20Reference) (Montant :type Float%20%28single-precision%29))
  (if (< (Variables|/Game/Blueprints/Personnages/Cody.Cody_C|GetSonic Personnage) 1e+02)
    (Variables|/Game/Blueprints/Personnages/Cody.Cody_C|SetSonic Personnage (+ (Variables|/Game/Blueprints/Personnages/Cody.Cody_C|GetSonic Personnage) Montant))
    (else
      ;[1 1 1] Mettre tous les cercle en normal + ajouter plus 1 au score
      (Default|ModeSonic Personnage))))

(fn AjouterPoints
  (params (Montant :type Integer) (Personnage :type Cody%20Object%20Reference))
  (if (Variables|/Game/Blueprints/Personnages/Cody.Cody_C|GetModeSonicActiver Personnage)
    (Variables|/Game/Blueprints/Personnages/Cody.Cody_C|SetScore Personnage (+ Montant 2))
    (else
      (Variables|/Game/Blueprints/Personnages/Cody.Cody_C|SetScore Personnage (+ Montant (Variables|Default|GetScore))))))

(fn DiminuerPoints
  (params (Montant :type Integer) (Personnage :type Cody%20Object%20Reference))
  (Variables|/Game/Blueprints/Personnages/Cody.Cody_C|SetScore Personnage (- Montant (Variables|Default|GetScore))))

(fn Conditions
  (params (CercleDetruis :type Boolean) (Danger :type Boolean))
  (Variables|Conditions|SetCercleDetruis CercleDetruis)
  (Variables|Conditions|SetCercleDangerSpawn Danger))

(fn ConditionsCercle
  (params (CercleNormal :type Boolean) (CercleBoost :type Boolean) (CercleBonus :type Boolean) (CercleDanger :type Boolean))
  (Variables|Conditions|SetCercleNormal CercleNormal)
  (Variables|Conditions|SetCercleBoost CercleBoost)
  (Variables|Conditions|SetCercleBonus CercleBonus)
  (Variables|Conditions|SetCercleDanger CercleDanger)
  (return))