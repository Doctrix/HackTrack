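; Platform actor whose static mesh moves steadily along negative local X and which destroys itself once the Cody character leaves it.
; Tick offsets the mesh by a fixed step each frame, without sweep or delta-time scaling.
; A Sphere overlap stores Cody and sets an in-zone flag, printing debug text on entry and exit.
; On exit, a short delay precedes destruction, skipped if Cody is back inside by then.
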(event OnComponentBeginOverlap(Sphere)
  (params (OverlappedComponent :type Primitive%20Component%20Object%20Reference) (OtherActor :type Actor%20Object%20Reference) (OtherComp :type Primitive%20Component%20Object%20Reference) (OtherBodyIndex :type Integer) (bFromSweep :type Boolean) (SweepResult :type Hit%20Result%20Structure%20%28by%20ref%29))
  (bind _ascody (Utilities|Casting|CastToCody OtherActor))
  (Variables|Default|SetPersonnage _ascody)
  (Variables|Default|SetEntrerDansLaZone true)
  (Development|PrintString "dedans"))

(event OnComponentEndOverlap(Sphere)
  (params (OverlappedComponent :type Primitive%20Component%20Object%20Reference) (OtherActor :type Actor%20Object%20Reference) (OtherComp :type Primitive%20Component%20Object%20Reference) (OtherBodyIndex :type Integer))
  (bind _ascody (Utilities|Casting|CastToCody OtherActor))
  (Variables|Default|SetPersonnage _ascody)
  (Variables|Default|SetEntrerDansLaZone false)
  (Development|PrintString "dehors")
  (Utilities|FlowControl|Delay 2.0)
  (if (not (Variables|Default|GetEntrerDansLaZone))
    (CallFunction|Detruire)))

(event Custom|Detruire
  (Actor|DestroyActor))

(event EventBeginPlay)

(event EventTick
  (params (DeltaSeconds :type Float%20%28single-precision%29))
  (Transformation|AddRelativeLocation (Variables|Default|GetStaticMesh) "-60.000000, 0, 0" false false))

(fn ConstructionScript)