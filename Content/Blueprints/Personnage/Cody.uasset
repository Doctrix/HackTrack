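; Cody is a character Blueprint that collects rings (Anneau) on the Action input and advances its Sphere component along local X every tick.
; On press, CastsRef fetches the first Anneau_Principal in the level; if its zone flag is set, the ring gives its reward, the HUD score updates and the ring is destroyed.
; An ActionActiver flag tracks the press, and the construction script assigns the Aura particle template.
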(event EventBeginPlay
  (Utilities|CastsRef)
  (bind _as0_hud (Utilities|Casting|CastTo0_HUD (HUD|GetHUD (Game|GetPlayerController 0))))
  (Variables|Default|SetHUD _as0_hud))

(event Collision|EventActorBeginOverlap
  (params (OtherActor :type Actor%20Object%20Reference)))

(event EventTick
  (params (DeltaSeconds :type Float%20%28single-precision%29))
  (Transformation|AddRelativeLocation (Variables|Default|GetSphere) (Math|Vector|MakeVector 1e+01 0.0 0.0) false false))

(event Input|ActionEvents|InputActionAction
  (params (Key :type Key%20Structure :default "None"))
  (bind _score (Variables|Default|GetScore))
  (bind _anneau (Variables|Default|GetAnneau))
  (bind _anneau_2 (Variables|Default|GetAnneau))
  (:Pressed
    (Variables|Default|SetActionActiver true)
    (Utilities|CastsRef)
    (Utilities|IsValid _anneau_2
      (:Is%20Valid
        (if (Variables|/Game/Blueprints/Anneau_Principal.Anneau_Principal_C|GetEntrerDansLaZone _anneau_2)
          (Utilities|IsValid _anneau
            (:Is%20Valid
              (Default|Recompense _anneau_2 (Variables|/Game/Blueprints/Anneau_Principal.Anneau_Principal_C|Gettype _anneau) _score)
              (Default|MajDuScore (Variables|/Game/Blueprints/Parametres/0_HUD.0_HUD_C|GetInterfaceDuJoueur (Variables|Default|GetHUD)) (Utilities|Text|ToText(Integer) _score))
              (Variables|Default|SetActionActiver false)
              (Default|Detruire _anneau_2)))))
      (:Is%20Not%20Valid
        (Utilities|FlowControl|Delay 1.0)
        (Variables|Default|SetActionActiver false))))
  (:Released
    (if (Variables|Default|GetActionActiver)
      (Variables|Default|SetActionActiver false))))

(fn ConstructionScript
  (Effects|Components|ParticleSystem|SetTemplate (Variables|Default|GetAura) (Variables|Default|GetP_Aura)))