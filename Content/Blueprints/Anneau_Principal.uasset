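; Main ring actor (Anneau) that drifts along local X by a random step each Tick and tracks when Cody enters its sphere.
; Its Type sets the color of dynamic M_Obstacle materials on its two meshes.
; Two seconds after Cody exits, it destroys itself unless re-entered.
; Recompense sets Cody's Score by Type but is not called here; the Ghost poseable-mesh helper is likewise uncalled.
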(event OnComponentBeginOverlap(Sphere)
  (params (OverlappedComponent :type Primitive%20Component%20Object%20Reference) (OtherActor :type Actor%20Object%20Reference) (OtherComp :type Primitive%20Component%20Object%20Reference) (OtherBodyIndex :type Integer) (bFromSweep :type Boolean) (SweepResult :type Hit%20Result%20Structure%20%28by%20ref%29))
  (bind _ascody (Utilities|Casting|CastToCody OtherActor))
  (Variables|Default|SetPersonnage _ascody)
  (Variables|Default|SetEntrerDansLaZone true))

(event OnComponentEndOverlap(Sphere)
  (params (OverlappedComponent :type Primitive%20Component%20Object%20Reference) (OtherActor :type Actor%20Object%20Reference) (OtherComp :type Primitive%20Component%20Object%20Reference) (OtherBodyIndex :type Integer))
  (bind _ascody (Utilities|Casting|CastToCody OtherActor))
  (Variables|Default|SetPersonnage _ascody)
  (Variables|Default|SetEntrerDansLaZone false)
  (Utilities|FlowControl|Delay 2.0)
  (if (not (Variables|Default|GetEntrerDansLaZone))
    (CallFunction|Detruire)))

(event Custom|Detruire
  (Components|Activation|SetAutoActivate (Variables|Default|GetParticleSystem) true)
  (Actor|DestroyActor))

(event EventBeginPlay
  (for _array_element (Utilities|Array|MakeArray (Variables|Default|GetStaticMesh) (Variables|Default|GetStaticMesh1))
    (bind _returnvalue (Rendering|Material|CreateDynamicMaterialInstance _array_element 0 "/Game/Materials/M_Obstacle.M_Obstacle" "None" :!class /Script/Engine.PrimitiveComponent))
    (Variables|Default|SetMaterialSM _returnvalue)
    (CallFunction|GestionParType)))

(event EventTick
  (params (DeltaSeconds :type Float%20%28single-precision%29))
  (Transformation|AddRelativeLocation (Variables|Default|GetAnneau) (Math|Vector|MakeVector (Math|Random|RandomFloatinRange (Variables|Default|GetVitesseDeDeplacementMin) (Variables|Default|GetVitesseDeDeplacementMax)) 0.0 0.0) false false))

(fn ConstructionScript
  (CallFunction|GestionParType))

(fn GestionParType
  (if (Utilities|Enum|Equal(Enum) (Variables|Default|Gettype) "NewEnumerator0")
    (bind _materialsm (Variables|Default|GetMaterialSM)
      (:then
        (Rendering|Material|SetVectorParameterValue _materialsm "Couleur" "(R=0.322917,G=0.492187,B=1.000000,A=1.000000)" :!class /Script/Engine.MaterialInstanceDynamic))
      (:else))
    (elif (Utilities|Enum|Equal(Enum) (Variables|Default|Gettype) "NewEnumerator1")
      (bind _materialsm_2 (Variables|Default|GetMaterialSM)
        (:then
          (Rendering|Material|SetVectorParameterValue _materialsm_2 "Couleur" "(R=0.000000,G=0.333333,B=0.059558,A=1.000000)" :!class /Script/Engine.MaterialInstanceDynamic))
        (:else))
      (elif (Utilities|Enum|Equal(Enum) (Variables|Default|Gettype) "NewEnumerator2")
        (bind _materialsm_3 (Variables|Default|GetMaterialSM)
          (:then
            (Rendering|Material|SetVectorParameterValue _materialsm_3 "Couleur" "(R=0.953206,G=1.000000,B=0.000000,A=1.000000)" :!class /Script/Engine.MaterialInstanceDynamic))
          (:else))
        (elif (Utilities|Enum|Equal(Enum) (Variables|Default|Gettype) "NewEnumerator3")
          (bind _materialsm_4 (Variables|Default|GetMaterialSM)
            (:then
              (Rendering|Material|SetVectorParameterValue _materialsm_4 "Couleur" "(R=1.000000,G=0.106452,B=0.000000,A=1.000000)" :!class /Script/Engine.MaterialInstanceDynamic))
            (:else)))))))

(fn Recompense
  (params (Type :type e_type%20Enum :default "NewEnumerator0") (Montant :type Integer))
  (bind _personnage (Variables|Default|GetPersonnage))
  (if (Utilities|Enum|Equal(Enum) Type "NewEnumerator0")
    (Variables|/Game/Blueprints/Personnage/Cody.Cody_C|SetScore _personnage (+ Montant (Variables|Default|GetScore)))
    (elif (Utilities|Enum|Equal(Enum) Type "NewEnumerator1")
      (Variables|/Game/Blueprints/Personnage/Cody.Cody_C|SetScore _personnage (+ Montant (Variables|Default|GetScore)))
      (elif (not (Utilities|Enum|Equal(Enum) Type "NewEnumerator2"))
        (if (Utilities|Enum|Equal(Enum) Type "NewEnumerator3")
          (Variables|/Game/Blueprints/Personnage/Cody.Cody_C|SetScore _personnage (- Montant (Variables|Default|GetScore))))))))

(fn Ghost
  (bind _returnvalue (AddComponent|AddPoseableMeshComponent true))
  (LocalVariables|SetL_Ghost _returnvalue))